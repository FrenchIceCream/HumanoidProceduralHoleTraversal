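; BP_AnimatedCharacter is a player-controlled Character that walks, sprints, looks and rotates through Enhanced Input.
; BeginPlay adds its mapping context and passes the scaled capsule height to ABP_AnimatedCharacter.
; Movement follows controller yaw, sprint switches the walk speed cap, and a separate action rotates the actor directly.
; A debug action slows global time while triggered and restores it when completed or canceled.
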(event `EnhancedInput|/Game/AnimatedCharacter/Input/IA_DebugTimeScale`
  (params (ActionValue :type "Vector2D Structure") (ElapsedSeconds :type "Float (double-precision)") (TriggeredSeconds :type "Float (double-precision)") (InputAction :type "InputAction Object Reference" :default "/Game/AnimatedCharacter/Input/IA_DebugTimeScale.IA_DebugTimeScale"))
  ; Handling Input
  (:`Triggered`
    (`GameplayStatics.SetGlobalTimeDilation` 0.1))
  (:`Canceled`
    (`GameplayStatics.SetGlobalTimeDilation` 1.0 :!label _label))
  (:`Completed`
    (goto _label)))

(event `EnhancedInput|/Game/AnimatedCharacter/Input/IA_Walk`
  (params (ActionValue :type "Vector2D Structure") (ElapsedSeconds :type "Float (double-precision)") (TriggeredSeconds :type "Float (double-precision)") (InputAction :type "InputAction Object Reference" :default "/Game/AnimatedCharacter/Input/IA_Walk.IA_Walk"))
  (bind (_x _y) (`KismetMathLibrary.BreakVector2D` ActionValue))
  (bind _returnvalue (`KismetMathLibrary.MakeRotator` 0.0 0.0 (.yaw (`self.GetControlRotation`))))
  ; Handling Input
  (:`Triggered`
    (`self.AddMovementInput` (`KismetMathLibrary.GetRightVector` _returnvalue) _x)
    (`self.AddMovementInput` (`KismetMathLibrary.GetForwardVector` _returnvalue) _y)))

(event `EnhancedInput|/Game/AnimatedCharacter/Input/IA_Look`
  (params (ActionValue :type "Vector2D Structure") (ElapsedSeconds :type "Float (double-precision)") (TriggeredSeconds :type "Float (double-precision)") (InputAction :type "InputAction Object Reference" :default "/Game/AnimatedCharacter/Input/IA_Look.IA_Look"))
  (bind (_x _y) (`KismetMathLibrary.BreakVector2D` ActionValue))
  ; Handling Input
  (:`Triggered`
    (`self.AddControllerYawInput` _x)
    (`self.AddControllerPitchInput` _y)))

(event `EnhancedInput|/Game/AnimatedCharacter/Input/IA_Sprint`
  (params (ActionValue :type Boolean) (ElapsedSeconds :type "Float (double-precision)") (TriggeredSeconds :type "Float (double-precision)") (InputAction :type "InputAction Object Reference" :default "/Game/AnimatedCharacter/Input/IA_Sprint.IA_Sprint"))
  (bind _charactermovement (`self.CharacterMovement`))
  ; Handling Input
  (:`Triggered`
    (set `CharacterMovementComponent.MaxWalkSpeed` 800.0 _charactermovement))
  (:`Canceled`
    (set `CharacterMovementComponent.MaxWalkSpeed` 200.0 _charactermovement :!label _label_2))
  (:`Completed`
    (goto _label_2)))

(event `EnhancedInput|/Game/AnimatedCharacter/Input/IA_Rotate`
  (params (ActionValue :type "Float (double-precision)") (ElapsedSeconds :type "Float (double-precision)") (TriggeredSeconds :type "Float (double-precision)") (InputAction :type "InputAction Object Reference" :default "/Game/AnimatedCharacter/Input/IA_Rotate.IA_Rotate"))
  ; Handling Input
  (:`Triggered`
    (`self.K2_AddActorLocalRotation` (`KismetMathLibrary.MakeRotator` 0.0 0.0 ActionValue))))

(event `self.ReceiveBeginPlay`
  (bind _asplayer_controller (cast `PlayerController` (`self.GetController`)))
  (message `EnhancedInputSubsystemInterface.AddMappingContext` (pcsubsystem `EnhancedInputLocalPlayerSubsystem` _asplayer_controller) "/Game/AnimatedCharacter/Input/IM_AnimatedCharacter.IM_AnimatedCharacter" 0 (struct))
  (bind _asabp_animated_character (cast `/Game/AnimatedCharacter/Animation/ABP_AnimatedCharacter` (`SkeletalMeshComponent.GetAnimInstance` (`self.Mesh`))))
  (set `/Game/AnimatedCharacter/Animation/ABP_AnimatedCharacter.CharacterHeight` (* (`CapsuleComponent.GetScaledCapsuleHalfHeight` (`self.CapsuleComponent`)) 2.0) _asabp_animated_character))

(fn `UserConstructionScript`)